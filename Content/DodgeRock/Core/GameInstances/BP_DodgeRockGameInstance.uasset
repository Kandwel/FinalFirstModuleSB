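; Game instance for DodgeRock that holds the selected game difficulty and the highest score.
; Simple setter and getter functions expose both values.
; The high score setter only overwrites the stored value when the new score is greater, and nothing here saves either value to disk.
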(fn SetGameDifficulty
  (params (GameDifficulty :type EGameDifficulty%20Enum :default "NewEnumerator0"))
  (Variables|Default|SetGameDifficulty GameDifficulty))

(fn GetGameDifficulty
  (return (Variables|Default|GetGameDifficulty)))

(fn SetHighScore
  (params (HighestScore :type Integer))
  (if (> HighestScore (CallFunction|GetHighScore))
    (Variables|Default|SetHighestScore HighestScore)))

(fn GetHighScore
  (return (Variables|Default|GetHighestScore)))