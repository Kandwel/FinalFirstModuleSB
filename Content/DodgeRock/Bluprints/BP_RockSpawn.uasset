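; BP_RockSpawn is a spawner that drops BP_Rock actors into the level at random points within its Box volume.
; On BeginPlay it reads the difficulty from BP_DodgeRockGameInstance and selects a damage value that rises with difficulty.
; SpawnRockInVolume randomizes X and Y inside the box, keeps the spawner's own height, and passes that damage to each rock as BaseDamage.
; Nothing in this Blueprint calls the spawn event itself.
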(event Custom|SpawnRockInVolume
  (bind _box (Variables|Default|GetBox))
  (bind _returnvalue (Transformation|GetWorldLocation _box))
  (bind _returnvalue_2 (Components|Box|GetScaledBoxExtent _box))
  (bind _returnvalue_3 (Math|Random|RandomPointinBoundingBox _returnvalue _returnvalue_2))
  (bind (_x _y) (Math|Vector|BreakVector _returnvalue_3))
  (Game|SpawnActorfromClass "/Game/DodgeRock/Bluprints/BP_Rock.BP_Rock_C" (Math|Transform|MakeTransform (Math|Vector|MakeVector _x _y (.Z (Math|Vector|BreakVector (Transformation|GetActorLocation))))) "AdjustIfPossibleButAlwaysSpawn" "OverrideRootScale" 0 (Variables|Default|GetRockDamageModifier) 0))

(event EventBeginPlay
  (bind _asbp_dodge_rock_game_instance (Utilities|Casting|CastToBP_DodgeRockGameInstance (Game|GetGameInstance)))
  (Variables|Default|SetRockDamageModifier (Utilities|Select :Index (Default|GetGameDifficulty _asbp_dodge_rock_game_instance) :NewEnumerator0 25.0 :NewEnumerator1 5e+01 :NewEnumerator2 1e+02)))

(fn ConstructionScript)