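; Healing pickup for DodgeRock that adds a fixed amount of health to the player character on contact.
; BeginPlay binds the actor hit event and caches the player character, whose health component is read on each Player-tagged hit.
; Health is added only when above zero and below full, with no clamp here, but the pickup destroys itself either way.
; Healing activates the character's Niagara effect, with deactivation behind a Delay on this soon-destroyed actor.
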(event Custom|OnActorHit_Event
  (params (SelfActor :type Actor%20Object%20Reference) (OtherActor :type Actor%20Object%20Reference) (NormalImpulse :type Vector) (Hit :type Hit%20Result%20Structure%20%28by%20ref%29))
  (if (Actor|ActorHasTag OtherActor "Player")
    (Variables|Default|SetHealth (Default|GetHealth (Variables|/Game/DodgeRock/Characters/BP_DodgeRockCharacter.BP_DodgeRockCharacter_C|GetBP_HelthComponent (Variables|Default|GetDodgeRockCharacter))))
    (Variables|Default|GetDodgeRockCharacter
      (:then
        (if (and (> (Variables|Default|GetHealth) 0.0) (< (Variables|Default|GetHealth) 1e+02))
          (Default|SetHealth (Variables|/Game/DodgeRock/Characters/BP_DodgeRockCharacter.BP_DodgeRockCharacter_C|GetBP_HelthComponent (Variables|Default|GetDodgeRockCharacter)) (+ (Variables|Default|GetHealth) 25.0))
          (CallFunction|PlayHealNiagara))
        (Actor|DestroyActor))
      (:else))))

(event Custom|PlayHealNiagara
  (bind _dodgerockcharacter (Variables|Default|GetDodgeRockCharacter)
    (:then
      (Components|Activation|SetActive (Variables|/Game/DodgeRock/Characters/BP_DodgeRockCharacter.BP_DodgeRockCharacter_C|GetNS_HealNiagara _dodgerockcharacter) true false)
      (Utilities|FlowControl|Delay 0.2)
      (Components|Activation|SetActive (Variables|/Game/DodgeRock/Characters/BP_DodgeRockCharacter.BP_DodgeRockCharacter_C|GetNS_HealNiagara _dodgerockcharacter) false false))
    (:else)))

(event EventBeginPlay
  (Utilities|FlowControl|Sequence
    (:then_0
      (Collision|BindEventtoOnActorHit (EventDispatchers|CreateEvent :!event Custom|OnActorHit_Event)))
    (:then_1
      (bind _asbp_dodge_rock_character (Utilities|Casting|CastToBP_DodgeRockCharacter (Game|GetPlayerCharacter 0)))
      (bind _output_get (Variables|Default|SetDodgeRockCharacter _asbp_dodge_rock_character))
      (Variables|Default|SetHealth (Default|GetHealth (Variables|/Game/DodgeRock/Characters/BP_DodgeRockCharacter.BP_DodgeRockCharacter_C|GetBP_HelthComponent _output_get))))))

(fn ConstructionScript)